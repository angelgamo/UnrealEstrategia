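; Enemy actor that walks a tile path to the tower and damages it on arrival.
; Each Tick it faces the next tile, moves forward and, within an arrival margin, advances to that tile's parent, following parent links toward the tower.
; At the tower it damages it through GMBBP, destroys itself and triggers a wave-end check.
; ReceiveDamage updates the health bar widget and destroys the enemy at zero health, also checking wave end.
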(event `self.ReceiveBeginPlay`
  (bind _asenemy_health_bar (cast `/Game/HUD/EnemyHealthBar` (`WidgetComponent.GetUserWidgetObject` (`self.HeathBar`))))
  (set `self.HeathBarWidgetREF` _asenemy_health_bar)
  (set `self.Health` 100))

(event `self.ReceiveTick`
  (params (DeltaSeconds :type "Float (single-precision)"))
  (`|ExecutionSequence`
    (:`then_0`
      (`self.LookAt`))
    (:`then_1`
      (`self.MoveForward` DeltaSeconds))
    (:`then_2`
      (`self.CheckDistance`))))

(fn `CheckDistance`
  (if (< (`KismetMathLibrary.Vector_Distance` (`SceneComponent.K2_GetComponentLocation` (`self.DefaultSceneRoot`)) (`self.NextTilePos`)) (`self.ArriveMargin`))
    (`self.GetNextTile`)))

(fn `GetNextTile`
  (bind _tile (`self.Tile`))
  (if (`/Game/BP/TileBP.isTower` _tile)
    (`KismetSystemLibrary.PrintString` "Enemy arrived to the tower")
    (`/Game/BP/GMBBP.DamageTower` (`self.GMBBP`) (`self.Damage`))
    (`self.K2_DestroyActor`)
    (`/Game/BP/GMBBP.CheckEndWave` (`self.GMBBP`))
    (else
      (bind _parent (`/Game/BP/TileBP.GetParent` _tile))
      (bind _output_get (set `self.Tile` _parent))
      (set `self.NextTilePos` (`SceneComponent.K2_GetComponentLocation` (`/Game/BP/TileBP.DefaultSceneRoot` _output_get))))))

(fn `GetTile`
  (if (`/Game/BP/TileBP.isTower` (`self.Tile`))
    (`KismetSystemLibrary.PrintString` "Enemy arrived to the towero")
    (`self.K2_DestroyActor`)
    (else
      (set `self.NextTilePos` (`SceneComponent.K2_GetComponentLocation` (`/Game/BP/TileBP.DefaultSceneRoot` (`self.Tile`)))))))

(fn `LookAt`
  (`self.K2_SetActorRotation` (`KismetMathLibrary.FindLookAtRotation` (`SceneComponent.K2_GetComponentLocation` (`self.DefaultSceneRoot`)) (`self.NextTilePos`))))

(fn `MoveForward`
  (params (delta :type "Float (double-precision)"))
  (`SceneComponent.K2_SetWorldLocation` (`self.DefaultSceneRoot`) (+ (* (`self.GetActorForwardVector`) (* delta (`self.Speed`))) (`SceneComponent.K2_GetComponentLocation` (`self.DefaultSceneRoot`))) false false))

(fn `ReceiveDamage`
  (params (Damage :type Integer))
  (bind _output_get (set `self.Health` (`KismetMathLibrary.Clamp` (- (`self.Health`) Damage) 0 100)))
  (set `/Game/HUD/EnemyHealthBar.Health` (`KismetMathLibrary.Conv_IntToDouble` _output_get) (`self.HeathBarWidgetREF`))
  (if (== (`self.Health`) 0)
    (`/Game/BP/GMBBP.CheckEndWave` (`self.GMBBP`))
    (`self.K2_DestroyActor`)))

(fn `UserConstructionScript`)