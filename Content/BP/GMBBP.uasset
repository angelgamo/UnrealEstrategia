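; Game manager for a tower defense with a growing tile path, handling startup, HUDs, gold, base health and restart.
; NewTile extends the path from the last tile's exit, rejecting candidates whose exit hits an occupied cell and falling back to a portal.
; Enemies spawn at the path's end, whose widget reappears when a wave ends.
; Selecting a tower tile opens the build HUD, and CreateTower spends gold to replace that tile with a tower.
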(event `self.ReceiveBeginPlay`
  (bind _gamehud (`self.GameHUD`))
  (`|ExecutionSequence`
    (:`then_0`
      (`self.SetPlayerControllerVars`)
      (`self.MakeTowerList`)
      (`self.AddHUD`)
      (bind _outactors (`GameplayStatics.GetAllActorsOfClass` "/Game/BP/PlayerBP.PlayerBP_C"))
      (bind _output_get (set `self.PlayerController` (`|GetArrayItem` _outactors)))
      (set `self.PlayerCamera` (`/Game/BP/PlayerBP.Camera` _output_get)))
    (:`then_1`
      (bind _returnvalue (`|SpawnActorFromClass` (`KismetArrayLibrary.Array_Random` (`self.TowerList`)) (`KismetMathLibrary.MakeTransform` (0.0 0.0 0.0)) "Undefined" "OverrideRootScale" null null))
      (`|ExecutionSequence`
        (:`then_0`
          (bind _output_get_2 (set `self.LastTile` _returnvalue))
          (bind _pos (`/Game/BP/TileBP.GetPos` _output_get_2))
          (`KismetSystemLibrary.PrintString` (`KismetStringLibrary.Concat_StrStr` "Tower Placed at " (`KismetStringLibrary.Conv_IntPointToString` _pos)))
          (`KismetArrayLibrary.Array_Add` (`self.Occupied`) _pos))
        (:`then_1`
          (bind _astower_1tile_bp (cast `/Game/BP/Tower/Tower1TileBP` _returnvalue)
            (:`then`
              (bind _astower_health_bar (cast `/Game/HUD/TowerHealthBar` (`WidgetComponent.GetWidget` (`/Game/BP/Tower/Tower1TileBP.HealthBar` _astower_1tile_bp))))
              (set `self.HealthBarWidgetREF` _astower_health_bar))
            (:`CastFailed`
              (bind _astower_2tile_bp (cast `/Game/BP/Tower/Tower2TileBP` _returnvalue))
              (bind _astower_health_bar_2 (cast `/Game/HUD/TowerHealthBar` (`WidgetComponent.GetWidget` (`/Game/BP/Tower/Tower2TileBP.HealthBar` _astower_2tile_bp))))
              (set `self.HealthBarWidgetREF` _astower_health_bar_2)))
          (bind _output_get_3 (set `self.Health` 20))
          (set `/Game/HUD/GameHUD.Health` _output_get_3 _gamehud)
          (bind _output_get_4 (set `self.Level` 1))
          (set `/Game/HUD/GameHUD.Level` _output_get_4 _gamehud)
          (bind _output_get_5 (set `self.Gold` 250))
          (set `/Game/HUD/GameHUD.Gold` _output_get_5 _gamehud))
        (:`then_2`
          (`SceneComponent.SetVisibility` (`/Game/BP/TileBP.Widget` _returnvalue) true false))))))

(fn `AddGold`
  (params (Gold :type Integer))
  (bind _output_get (set `self.Gold` (+ Gold (`self.Gold`))))
  (set `/Game/HUD/GameHUD.Gold` _output_get (`self.GameHUD`)))

(fn `AddHUD`
  (`|ExecutionSequence`
    (:`then_0`
      (bind _returnvalue (`|CreateWidget` "/Game/HUD/TowersHUDBP.TowersHUDBP_C"))
      (if (not (`Widget.IsInViewport` _returnvalue))
        (`UserWidget.AddToViewport` _returnvalue 0)
        (`Widget.SetVisibility` _returnvalue "Hidden")
        (set `self.HUD` _returnvalue)))
    (:`then_1`
      (bind _returnvalue_2 (`|CreateWidget` "/Game/HUD/ResetHUD.ResetHUD_C"))
      (if (not (`Widget.IsInViewport` _returnvalue_2))
        (`UserWidget.AddToViewport` _returnvalue_2 0)
        (`Widget.SetVisibility` _returnvalue_2 "Hidden")
        (set `self.ResetHud` _returnvalue_2)))
    (:`then_2`
      (bind _returnvalue_3 (`|CreateWidget` "/Game/HUD/GameHUD.GameHUD_C"))
      (if (not (`Widget.IsInViewport` _returnvalue_3))
        (`UserWidget.AddToViewport` _returnvalue_3 0)
        (set `self.GameHUD` _returnvalue_3)))))

(fn `CheckEndWave`
  (bind _outactors (`GameplayStatics.GetAllActorsOfClass` "/Game/BP/EnemyBP.EnemyBP_C"))
  (if (<= (`KismetArrayLibrary.Array_Length` _outactors) 1)
    (`KismetSystemLibrary.PrintString` "EndWave")
    (`SceneComponent.SetVisibility` (`/Game/BP/TileBP.Widget` (`self.LastTile`)) true false)))

(fn `Create Tower`
  (params (inTow :type "/Game/BP/TowerTile/Tow Object Reference"))
  (bind _actualtilebp (`self.actualTileBP`))
  (bind _gold (`self.Gold`))
  (bind _gold_2 (`/Game/BP/TowerTile/Tow.Gold` inTow))
  (`/Engine/EditorBlueprintResources/StandardMacros.IsValid` _actualtilebp
    (:`Is Valid`
      (if (>= _gold _gold_2)
        (bind _output_get (set `self.Gold` (- _gold _gold_2)))
        (set `/Game/HUD/GameHUD.Gold` _output_get (`self.GameHUD`))
        (`|ExecutionSequence`
          (:`then_0`
            (bind _returnvalue (`|SpawnActorFromClass` "/Game/BP/TowerTile/TowWrapper.TowWrapper_C" (`self.GetTransform` _actualtilebp) "AlwaysSpawn" "OverrideRootScale" null null))
            (`/Game/BP/TowerTile/TowWrapper.SetTower` _returnvalue inTow)
            (`Widget.SetVisibility` (`self.HUD`) "Hidden")
            (set `/Game/BP/PlayerBP.checkMouse` false (`self.PlayerController`))
            (`ParticleSystemComponent.SetTemplate` (`/Game/BP/TowerTile/TowWrapper.Particles` _returnvalue) (`/Game/BP/TowerTile/Tow.ParticlesTemplate` inTow)))
          (:`then_1`
            (`self.K2_DestroyActor` _actualtilebp)))))))

(fn `DamageTower`
  (params (Damage :type Integer))
  (bind _output_get (set `self.Health` (`KismetMathLibrary.Clamp` (- (stale _output_get) Damage) 0 100)))
  (bind _output_get_2 (set `/Game/HUD/TowerHealthBar.Health` _output_get (`self.HealthBarWidgetREF`)))
  (set `/Game/HUD/GameHUD.Health` _output_get_2 (`self.GameHUD`))
  (if (== _output_get 0)
    (`Widget.SetVisibility` (`self.ResetHud`) "Visible")
    (`Widget.SetVisibility` (`self.HUD`) "Hidden")))

(fn `GetRandomTile`
  (params (last :type Integer))
  (returns (tile :type "/Game/BP/TileBP Class Reference") (index :type Integer))
  (bind (_outitem _outindex) (`KismetArrayLibrary.Array_Random` (`self.list_0`)))
  (bind (_outitem_2 _outindex_2) (`KismetArrayLibrary.Array_Random` (`self.list_1`)))
  (bind (_outitem_3 _outindex_3) (`KismetArrayLibrary.Array_Random` (`self.list_2`)))
  (bind (_outitem_4 _outindex_4) (`KismetArrayLibrary.Array_Random` (`self.list_3`)))
  (bind _exit (`/Game/BP/TileBP.Exit` (`self.LastTile`)))
  (bind _exit_2 (`/Game/BP/TileBP.Exit` (`self.LastTile`)))
  (if (== last -1)
    (if (== _exit 0)
      (return _outitem _outindex)
      (elif (== _exit 1)
        (return _outitem_2 _outindex_2)
        (elif (== _exit 2)
          (return _outitem_3 _outindex_3)
          (elif (== _exit 3)
            (return _outitem_4 _outindex_4)))))
    (elif (== _exit_2 0)
      (return (`|GetArrayItem` (`self.list_0`) last) last)
      (elif (== _exit_2 1)
        (return (`|GetArrayItem` (`self.list_1`) last) last)
        (elif (== _exit_2 2)
          (return (`|GetArrayItem` (`self.list_2`) last) last)
          (elif (== _exit_2 3)
            (return (`|GetArrayItem` (`self.list_3`) last) last)))))))

(fn `MakeTowerList`
  (bind _towlist (`self.towList`))
  (bind _returnvalue (`AddComponent|NODE_AddTower1-0`))
  (`KismetArrayLibrary.Array_Add` _towlist _returnvalue)
  (bind _returnvalue_2 (`AddComponent|NODE_AddTesla-1`))
  (`KismetArrayLibrary.Array_Add` _towlist _returnvalue_2))

(fn `MouseClick`
  (bind _actualtilebp (`self.actualTileBP`))
  (bind _returnvalue (`WidgetLayoutLibrary.GetMousePositionOnViewport`))
  (bind _returnvalue_2 (`KismetMathLibrary.Conv_Vector2DToIntPoint` _returnvalue))
  (if (`KismetMathLibrary.Equal_IntPointIntPoint` (`self.lastMouse`) _returnvalue_2)
    (set `self.lastMouse` _returnvalue_2)
    (`Widget.SetVisibility` (`self.HUD`) "Hidden")
    (set `/Game/BP/PlayerBP.checkMouse` false (`self.PlayerController`))
    (`/Engine/EditorBlueprintResources/StandardMacros.IsValid` _actualtilebp
      (:`Is Valid`
        (`/Game/BP/TowerTileBP.SetColor` _actualtilebp (`self.baseColor`))
        (set `self.actualTileBP` null)
        (set `self.lastMouse` (struct))))
    (else
      (set `self.lastMouse` _returnvalue_2))))

(fn `NewEnemy`
  (bind _returnvalue (* (`self.TileSize`) 0.5))
  (bind _returnvalue_2 (`SceneComponent.K2_GetComponentLocation` (`/Game/BP/TileBP.DefaultSceneRoot` (`self.LastTile`))))
  (if (`/Game/BP/TileBP.isPortal` (`self.LastTile`))
    (bind _returnvalue_3 (`|SpawnActorFromClass` (`self.Enemy`) (`KismetMathLibrary.MakeTransform` _returnvalue_2) "Undefined" "OverrideRootScale" null null))
    (set `/Game/BP/EnemyBP.Tile` (`self.LastTile`) _returnvalue_3)
    (set `/Game/BP/EnemyBP.GMBBP` self _returnvalue_3)
    (`/Game/BP/EnemyBP.GetTile` _returnvalue_3)
    (else
      (bind _returnvalue_4 (`|SpawnActorFromClass` (`self.Enemy`) (`KismetMathLibrary.MakeTransform` (+ _returnvalue_2 (* (`|GetArrayItem` (`self.Sides`) (`/Game/BP/TileBP.Exit` (`self.LastTile`))) (`KismetMathLibrary.MakeVector2D` _returnvalue _returnvalue)))) "Undefined" "OverrideRootScale" null null))
      (set `/Game/BP/EnemyBP.Tile` (`self.LastTile`) _returnvalue_4)
      (set `/Game/BP/EnemyBP.GMBBP` self _returnvalue_4)
      (`/Game/BP/EnemyBP.GetTile` _returnvalue_4))))

(fn `NewTile`
  (bind _tilesize (`self.TileSize`))
  (bind _returnvalue (+ (`SceneComponent.K2_GetComponentLocation` (`/Game/BP/TileBP.DefaultSceneRoot` (`self.LastTile`))) (* (`|GetArrayItem` (`self.Sides`) (`/Game/BP/TileBP.Exit` (`self.LastTile`))) (`KismetMathLibrary.MakeVector2D` _tilesize _tilesize))))
  (set `self.isTilePlaced` false)
  (if (not (`/Game/BP/TileBP.isPortal` (`self.LastTile`)))
    (set `self.temp` -1)
    (for _ (range 4)
      (bind (_tile _index) (`self.GetRandomTile` (`self.temp`)))
      (bind _result (`/Engine/EditorBlueprintResources/StandardMacros.IncrementInt` _index)
        (:`  `
          (set `self.temp` (mod _result 3))
          (bind _returnvalue_2 (`|SpawnActorFromClass` _tile (`KismetMathLibrary.MakeTransform` _returnvalue) "AlwaysSpawn" "OverrideRootScale" null null))
          (bind _pos (`/Game/BP/TileBP.GetPos` _returnvalue_2))
          (`self.CanPlace` _pos (`/Game/BP/TileBP.Exit` _returnvalue_2)
            (:`True`
              ;[0.4547 0.577 1] add and print created tile pos
              (bind _pos_2 (`/Game/BP/TileBP.GetPos` _returnvalue_2))
              (`KismetArrayLibrary.Array_Add` (`self.Occupied`) _pos_2)
              (`KismetSystemLibrary.PrintString` (`KismetStringLibrary.Concat_StrStr` "Tile Placed at" (`KismetStringLibrary.Conv_IntPointToString` _pos_2)))
              ;[1 0.4328 0.8652] set tile parent var
              (set `/Game/BP/TileBP.TileParent` (`self.LastTile`) _returnvalue_2)
              ;[1 0.753 0.4366] set last tile
              (set `self.LastTile` _returnvalue_2)
              (set `self.isTilePlaced` true)
              (break))
            (:`False`
              (`self.K2_DestroyActor` _returnvalue_2))))))
    (if (not (`self.isTilePlaced`))
      (bind _returnvalue_3 (`|SpawnActorFromClass` (`|GetArrayItem` (`self.PortalList`) (`/Game/BP/TileBP.Exit` (`self.LastTile`))) (`KismetMathLibrary.MakeTransform` _returnvalue) "AlwaysSpawn" "OverrideRootScale" null null))
      ;[0.4547 0.577 1] add and print created tile pos
      (bind _pos_3 (`/Game/BP/TileBP.GetPos` _returnvalue_3))
      (`KismetArrayLibrary.Array_Add` (`self.Occupied`) _pos_3)
      (`KismetSystemLibrary.PrintString` (`KismetStringLibrary.Concat_StrStr` "Tile Placed at" (`KismetStringLibrary.Conv_IntPointToString` _pos_3)))
      ;[1 0.4328 0.8652] set tile parent var
      (set `/Game/BP/TileBP.TileParent` (`self.LastTile`) _returnvalue_3)
      ;[1 0.753 0.4366] set last tile
      (set `self.LastTile` _returnvalue_3))))

(fn `OnClickTowerTileBP`
  (params (TowerTileTarget :type "/Game/BP/TowerTileBP Object Reference"))
  (bind _playercontroller (`self.PlayerController`))
  (bind _output_get (set `self.lastTileBP` (`self.actualTileBP`)))
  (`/Engine/EditorBlueprintResources/StandardMacros.IsValid` _output_get
    (:`Is Valid`
      (`self.OnDeselectTowerTileBP` _output_get)
      (`/Game/BP/TowerTileBP.SetColor` _output_get (`self.baseColor`)))
    (:`Is Not Valid`
      _))
  (bind _output_get_2 (set `self.actualTileBP` TowerTileTarget))
  (`/Game/BP/TowerTileBP.SetColor` _output_get_2 (`self.selectedColor`))
  (`Widget.SetVisibility` (`self.HUD`) "Visible")
  (set `/Game/BP/PlayerBP.checkMouse` true _playercontroller)
  (set `/Game/BP/PlayerBP.justPressed` true _playercontroller))

(fn `OnDeselectTowerTileBP`
  (params (TowerTileTarget :type "/Game/BP/TowerTileBP Object Reference"))
  (if (not (and (== TowerTileTarget (`self.actualTileBP`)) (`KismetMathLibrary.LinearColor_IsNearEqual` (`PaperSpriteComponent.SpriteColor` (`/Game/BP/TowerTileBP.PaperSprite` TowerTileTarget)) (`self.selectedColor`))))
    (`/Game/BP/TowerTileBP.SetColor` TowerTileTarget (`self.baseColor`))))

(fn `OnHoverTowerTileBP`
  (params (TowerTIleTarget :type "/Game/BP/TowerTileBP Object Reference"))
  (if (not (== TowerTIleTarget (`self.actualTileBP`)))
    (`/Game/BP/TowerTileBP.SetColor` TowerTIleTarget (`self.hoverColor`))))

(fn `Restart`
  (bind _returnvalue (`GameplayStatics.GetCurrentLevelName` true))
  (`GameplayStatics.OpenLevel` (`KismetStringLibrary.Conv_StringToName` _returnvalue)))

(fn `SetPlayerControllerVars`
  (bind _returnvalue (`GameplayStatics.GetPlayerController` 0))
  (set `PlayerController.bShowMouseCursor` true _returnvalue)
  (set `PlayerController.bEnableClickEvents` true _returnvalue)
  (set `PlayerController.bEnableMouseOverEvents` true _returnvalue)
  (set `PlayerController.bEnableTouchOverEvents` true _returnvalue))

(fn `UserConstructionScript`)