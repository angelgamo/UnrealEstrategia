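; Player Blueprint that pans the camera and forwards player input to the GMBBP game mode.
; Input flags drive Tick, which picks fast or slow velocity and moves the Camera along world XY diagonals via MoveCamera, which swaps its X and Y inputs.
; Action keys call NewTile and NewEnemy on the game mode.
; Left mouse press and release call MouseClick when CheckMouse allows, except a press that clears JustPressed.
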(event `self.ReceiveBeginPlay`
  (bind _asgmbbp (cast `/Game/BP/GMBBP` (`GameplayStatics.GetGameMode`)))
  (set `self.GMBBP` _asgmbbp))

(event `self.ReceiveTick`
  (params (DeltaSeconds :type "Float (single-precision)"))
  (bind _returnvalue (* DeltaSeconds (`self.CameraVelocity`)))
  (bind _returnvalue_2 (* _returnvalue -1.0))
  (`|ExecutionSequence`
    (:`then_0`
      (if (`self.CamFast`)
        (set `self.CameraVelocity` (`self.CameraVelocityFast`))
        (else
          (set `self.CameraVelocity` (`self.CameraVelocitySlow`)))))
    (:`then_1`
      (if (`self.CamUp`)
        (`self.MoveCamera` _returnvalue_2 _returnvalue)
        (elif (`self.CampDown`)
          (`self.MoveCamera` _returnvalue _returnvalue_2))))
    (:`then_2`
      (if (`self.CamLeft`)
        (`self.MoveCamera` _returnvalue_2 _returnvalue_2)
        (elif (`self.CamRight`)
          (`self.MoveCamera` _returnvalue _returnvalue))))))

(event `InputAction|CameraUp`
  (params (Key :type "Key Structure"))
  (:`Pressed`
    (set `self.CamUp` true))
  (:`Released`
    (set `self.CamUp` false)))

(event `InputAction|CameraDown`
  (params (Key :type "Key Structure"))
  (:`Pressed`
    (set `self.CampDown` true))
  (:`Released`
    (set `self.CampDown` false)))

(event `InputAction|CameraLeft`
  (params (Key :type "Key Structure"))
  (:`Pressed`
    (set `self.CamLeft` true))
  (:`Released`
    (set `self.CamLeft` false)))

(event `InputAction|CameraRight`
  (params (Key :type "Key Structure"))
  (:`Pressed`
    (set `self.CamRight` true))
  (:`Released`
    (set `self.CamRight` false)))

(event `InputAction|CameraFast`
  (params (Key :type "Key Structure"))
  (:`Pressed`
    (set `self.CamFast` true))
  (:`Released`
    (set `self.CamFast` false)))

(event `InputAction|action1`
  (params (Key :type "Key Structure"))
  (:`Pressed`
    (`/Game/BP/GMBBP.NewTile` (`self.GMBBP`))))

(event `InputAction|action2`
  (params (Key :type "Key Structure"))
  (:`Pressed`
    (`/Game/BP/GMBBP.NewEnemy` (`self.GMBBP`))))

(event `Key|LeftMouseButton`
  (params (Key :type "Key Structure"))
  (:`Pressed`
    (if (`self.justPressed`)
      (set `self.justPressed` false)
      (else
        (if (`self.checkMouse`) :!label _label
          (`/Game/BP/GMBBP.MouseClick` (`self.GMBBP`))))))
  (:`Released`
    (goto _label)))

(fn `MoveCamera`
  (params (X :type "Float (double-precision)") (Y :type "Float (double-precision)"))
  (`SceneComponent.K2_SetWorldLocation` (`self.Camera`) (`KismetMathLibrary.MakeVector` (+ Y (.x (`SceneComponent.K2_GetComponentLocation` (`self.Camera`)))) (+ X (.y (`SceneComponent.K2_GetComponentLocation` (`self.Camera`)))) (.z (`SceneComponent.K2_GetComponentLocation` (`self.Camera`)))) false false))

(fn `UserConstructionScript`)