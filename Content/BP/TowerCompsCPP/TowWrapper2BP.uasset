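; Tower wrapper actor that takes on a tower type at runtime from a supplied tower component.
; SetTower adds a new component of that component's class, passes it the GIMP reference, marks it active and links it back to this actor.
; The actor's static mesh then comes from the new component's tower mesh.
; The construction script stores the Particles component in MParicleSys.
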(fn `SetTower`
  (params (TowerComp :type "Tow2 Object Reference") (GIMP :type "GIMP Object Reference"))
  (bind _returnvalue (`|AddComponentByClass` self (`GameplayStatics.GetObjectClass` TowerComp)))
  (bind _output_get (set `self.TowerComp` _returnvalue))
  (set `Tow2.aguinp` GIMP _output_get)
  (set `Tow2.towerActive` true _output_get)
  (set `Tow2.selfActor` self _output_get)
  (`StaticMeshComponent.SetStaticMesh` (`self.StaticMesh`) (`Tow2.TowMesh` _output_get)))

(fn `UserConstructionScript`
  (set `self.mParicleSys` (`self.Particles`)))